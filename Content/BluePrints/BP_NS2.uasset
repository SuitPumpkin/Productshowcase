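; BP_NS2 is a console model actor with an animated exploded view that slides its left and right parts between armed and exploded positions.
; AlternarArmado, also bound to the F key and called on BeginPlay, flips IsExploted and plays or reverses TL_Explode.
; The timeline's alpha lerps both parts' relative locations with sweep enabled.
; OcultarConsola and MostrarConsola events hide and show the whole actor.
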(event `Alternar Armado`
  (if (`self.IsExploted`) :!label _label
    (set `self.IsExploted` false)
    (bind (_direction _alpha) (`Timeline|TL_Explode` :`NewTime` 1.0 :!via `Reverse` :!label _label_2)
      (:`Update`
        (`SceneComponent.K2_SetRelativeLocation` (`self.NS2_Left`) (`KismetMathLibrary.VLerp` (`self.Left_Armed_Pos`) (`self.Left_Exploded_Pos`) _alpha) true false)
        (`SceneComponent.K2_SetRelativeLocation` (`self.NS2_Right`) (`KismetMathLibrary.VLerp` (`self.Right_Armed_Pos`) (`self.Right_Exploded_Pos`) _alpha) true false)))
    (else
      (set `self.IsExploted` true)
      (goto _label_2))))

(event `Key|F`
  (params (Key :type "Key Structure"))
  (:`Pressed`
    (goto _label)))

(event `self.ReceiveBeginPlay`
  (`self.Alternar Armado`)
  (goto _label_2 :!via `SetNewTime`))

(event `Ocultar Consola`
  (`self.SetActorHiddenInGame` true))

(event `Mostrar Consola`
  (`self.SetActorHiddenInGame` false))

(fn `UserConstructionScript`)