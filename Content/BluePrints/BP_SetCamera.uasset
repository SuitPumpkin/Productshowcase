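; Camera and background manager that switches the player's view between orbit, front and back cameras and recolors the backdrop.
; On BeginPlay it adds the WBP_ControlCamaras widget, shows the cursor, starts on BP_CameraOrbit and applies one dynamic background material to every StaticMeshActor.
; Flag-guarded events, also bound to keys 1-3, change the view target, calling HacerZoom for front and back.
; Similar events set blue, green or orange gradient colors.
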(event `self.ReceiveBeginPlay`
  (bind _returnvalue (`|CreateWidget` "/Game/UI/WBP_ControlCamaras.WBP_ControlCamaras_C"))
  (`UserWidget.AddToViewport` _returnvalue 0)
  (bind _returnvalue_2 (`InputDeviceLibrary.GetPlayerControllerFromInputDevice` (struct)))
  (set `PlayerController.bShowMouseCursor` true _returnvalue_2)
  (bind _returnvalue_3 (`GameplayStatics.GetActorOfClass` "/Game/BluePrints/BP_CameraBack.BP_CameraBack_C"))
  (set `self.CamBack` _returnvalue_3)
  (bind _returnvalue_4 (`GameplayStatics.GetActorOfClass` "/Game/BluePrints/BP_CameraFront.BP_CameraFront_C"))
  (set `self.CamFront` _returnvalue_4)
  (bind _returnvalue_5 (`GameplayStatics.GetActorOfClass` "/Game/BluePrints/BP_CameraOrbit.BP_CameraOrbit_C"))
  (`PlayerController.SetViewTargetWithBlend` (`GameplayStatics.GetPlayerController` 0) _returnvalue_5 0.0 "VTBlend_Linear" 0.0 false)
  (bind _returnvalue_6 (`GameplayStatics.GetActorOfClass` "/Script/Engine.StaticMeshActor"))
  (bind _returnvalue_7 (`PrimitiveComponent.CreateDynamicMaterialInstance` (`StaticMeshActor.StaticMeshComponent` _returnvalue_6) 1 "/Game/Materiales/MI_Background_Inst.MI_Background_Inst" "None"))
  (bind _output_get (set `self.MI_Background_Dynamic` _returnvalue_7))
  (bind _outactors (`GameplayStatics.GetAllActorsOfClass` "/Script/Engine.StaticMeshActor"))
  (for _array_element _outactors
    (bind _staticmeshcomponent (`StaticMeshActor.StaticMeshComponent` _array_element))
    (`PrimitiveComponent.SetMaterial` _staticmeshcomponent 1 _output_get)
    (`PrimitiveComponent.SetMaterial` _staticmeshcomponent 2 _output_get)))

(event `CambiarOrbital`
  (if (not (`self.IsOrbital`)) :!label _label
    (bind _returnvalue (`GameplayStatics.GetActorOfClass` "/Game/BluePrints/BP_CameraOrbit.BP_CameraOrbit_C"))
    (`PlayerController.SetViewTargetWithBlend` (`GameplayStatics.GetPlayerController` 0) _returnvalue 0.0 "VTBlend_Linear" 0.0 false)
    (set `self.IsOrbital` true)
    (set `self.IsFrontal` false)
    (set `self.IsBack` false)))

(event `Key|One`
  (params (Key :type "Key Structure"))
  (:`Pressed`
    (goto _label)))

(event `CambiarFrontal`
  (if (not (`self.IsFrontal`)) :!label _label_2
    (bind _returnvalue (`GameplayStatics.GetActorOfClass` "/Game/BluePrints/BP_CameraFront.BP_CameraFront_C"))
    (`/Game/BluePrints/BP_CameraFront.HacerZoom` (`self.CamFront`))
    (`PlayerController.SetViewTargetWithBlend` (`GameplayStatics.GetPlayerController` 0) _returnvalue 0.0 "VTBlend_Linear" 0.0 false)
    (set `self.IsOrbital` false)
    (set `self.IsFrontal` true)
    (set `self.IsBack` false)))

(event `Key|Two`
  (params (Key :type "Key Structure"))
  (:`Pressed`
    (goto _label_2)))

(event `CambiarTrasera`
  (if (not (`self.IsBack`)) :!label _label_3
    (bind _returnvalue (`GameplayStatics.GetActorOfClass` "/Game/BluePrints/BP_CameraBack.BP_CameraBack_C"))
    (`/Game/BluePrints/BP_CameraBack.HacerZoom` (`self.CamBack`))
    (`PlayerController.SetViewTargetWithBlend` (`GameplayStatics.GetPlayerController` 0) _returnvalue 0.0 "VTBlend_Linear" 0.0 false)
    (set `self.IsOrbital` false)
    (set `self.IsFrontal` false)
    (set `self.IsBack` true)))

(event `Key|Three`
  (params (Key :type "Key Structure"))
  (:`Pressed`
    (goto _label_3)))

(event `FondoAzul`
  (bind _mi_background_dynamic (`self.MI_Background_Dynamic`))
  (if (not (`self.ColorBlue`))
    (`MaterialInstanceDynamic.SetVectorParameterValue` _mi_background_dynamic "Color_Top" (struct :`G` 0.904661 :`B` 1.0 :`A` 1.0))
    (`MaterialInstanceDynamic.SetVectorParameterValue` _mi_background_dynamic "Color_Bottom" (struct :`R` 0.076185 :`G` 0.201556 :`B` 1.0 :`A` 1.0))
    (set `self.ColorGreen` false)
    (set `self.ColorOrange` false)
    (set `self.ColorBlue` true)))

(event `FondoVerde`
  (bind _mi_background_dynamic (`self.MI_Background_Dynamic`))
  (if (not (`self.ColorGreen`))
    (`MaterialInstanceDynamic.SetVectorParameterValue` _mi_background_dynamic "Color_Top" (struct :`R` 0.171126 :`G` 1.0 :`B` 0.146875 :`A` 1.0))
    (`MaterialInstanceDynamic.SetVectorParameterValue` _mi_background_dynamic "Color_Bottom" (struct :`R` 0.067656 :`G` 0.244792 :`B` 0.062473 :`A` 1.0))
    (set `self.ColorGreen` true)
    (set `self.ColorOrange` false)
    (set `self.ColorBlue` false)))

(event `FondoNaranja`
  (bind _mi_background_dynamic (`self.MI_Background_Dynamic`))
  (if (not (`self.ColorOrange`))
    (`MaterialInstanceDynamic.SetVectorParameterValue` _mi_background_dynamic "Color_Top" (struct :`R` 1.0 :`G` 0.428691 :`A` 1.0))
    (`MaterialInstanceDynamic.SetVectorParameterValue` _mi_background_dynamic "Color_Bottom" (struct :`R` 0.307292 :`G` 0.131733 :`A` 1.0))
    (set `self.ColorGreen` false)
    (set `self.ColorOrange` true)
    (set `self.ColorBlue` false)))

(fn `UserConstructionScript`)