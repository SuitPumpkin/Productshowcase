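; Poseable studio C-stand prop with a gobo arm and an optional fluorescent light, configured entirely in the construction script with no runtime logic.
; Variables offset the components: one height value raises two telescoping rods in clamped stages, while others pose the bar clamps, arm and mount rotator.
; Lock handles spin automatically through range-mapped height and angle values.
; A toggle shows the light, whose tube gets a dynamic material for emissive color, intensity and tip darkening.
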(fn `UserConstructionScript`
  (`|ExecutionSequence`
    (:`then_0`
      (`SceneComponent.K2_AddWorldTransform` (`self.CTR01_InnerRod_A`) (`KismetMathLibrary.MakeTransform` (`KismetMathLibrary.MakeVector` 0.0 0.0 (+ 0.0 (`KismetMathLibrary.FClamp` (`self.01_ALL Rod Height`) 0.0 45.0)))) false false)
      (`SceneComponent.K2_AddWorldTransform` (`self.CTR02_InnerRod_B`) (`KismetMathLibrary.MakeTransform` (`KismetMathLibrary.MakeVector` 0.0 0.0 (+ 0.0 (`KismetMathLibrary.FClamp` (- (`self.01_ALL Rod Height`) 45.0) 0.0 40.0)))) false false)
      (`SceneComponent.K2_AddRelativeRotation` (`self.CTR03_BarClamp_Main`) (`KismetMathLibrary.MakeRotator` 0.0 (+ 0.0 (`self.02_BarClamp_Main_Angle`))) false false)
      (`SceneComponent.K2_AddRelativeLocation` (`self.CTR04_GoboArm`) (`KismetMathLibrary.MakeVector` (+ 0.0 (`self.03_GoboArm_Position`))) false false)
      (`SceneComponent.K2_AddRelativeRotation` (`self.CTR05_BarClamp_Tip`) (`KismetMathLibrary.MakeRotator` 0.0 (+ 0.0 (`self.04_BarClamp_Tip_Angle`))) false false)
      (`SceneComponent.K2_AddRelativeRotation` (`self.CTR06_Mount_Rotator`) (`self.05_Mount_Rotator`) false false))
    (:`then_1`
      (`SceneComponent.K2_AddRelativeRotation` (`self.CTR07_LockHandle_01`) (`KismetMathLibrary.MakeRotator` 0.0 (+ 0.0 (`KismetMathLibrary.MapRangeClamped` (`self.01_ALL Rod Height`) 0.0 45.0 0.0 720.0))) false false)
      (`SceneComponent.K2_AddRelativeRotation` (`self.CTR08_LockHandle_02`) (`KismetMathLibrary.MakeRotator` 0.0 (+ 0.0 (`KismetMathLibrary.MapRangeClamped` (`self.01_ALL Rod Height`) 46.0 90.0 0.0 720.0))) false false)
      (`SceneComponent.K2_AddRelativeRotation` (`self.CTR09_LockHandle_03`) (`KismetMathLibrary.MakeRotator` 0.0 (+ 0.0 (`KismetMathLibrary.MapRangeClamped` (`self.02_BarClamp_Main_Angle`) -71.0 85.0 0.0 720.0))) false false)
      (`SceneComponent.K2_AddRelativeRotation` (`self.CTR10_LockHandle_04`) (`KismetMathLibrary.MakeRotator` 0.0 (+ 0.0 (`KismetMathLibrary.MapRangeClamped` (`self.04_BarClamp_Tip_Angle`) -360.0 360.0 0.0 360.0))) false false))
    (:`then_2`
      (`SceneComponent.SetVisibility` (`self.SM_FluorescentLight`) (`self.UseFluorescentLight`) false)
      (`SceneComponent.SetVisibility` (`self.SM_FluorescentLight_Tube`) (`self.UseFluorescentLight`) false)
      (bind _returnvalue (`PrimitiveComponent.CreateDynamicMaterialInstance` (`self.SM_FluorescentLight_Tube`) 0 "/Game/Studios/Models/FluorescentLight/MI_FluorescentLight_Em.MI_FluorescentLight_Em" "None"))
      (`MaterialInstanceDynamic.SetScalarParameterValue` _returnvalue "DarkenLightTip" (`self.DarkenLightTip`))
      (`MaterialInstanceDynamic.SetScalarParameterValue` _returnvalue "Emissive Mult" (`self.Emissive Mult`))
      (`MaterialInstanceDynamic.SetVectorParameterValue` _returnvalue "EmissiveColor" (`self.EmissiveColor`)))))